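; VR player pawn for a repair game: clearing all defects wins, running out of energy loses.
; Tick applies the current charge or drain rate to energy and triggers the end widgets and delayed level loads.
; The right trigger capsule-traces for IF_VRInteraction actors, repairing them after a particle-backed delay.
; It also handles camera-relative movement, left-grip sphere-overlap grabbing through messages, and a toggled menu using widget interaction.
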(event `self.ReceiveBeginPlay`
  (set `self.Is charging` (`self.Uncharging speed`)))

(event `Lose`
  (`SceneComponent.SetHiddenInGame` (`self.LoseWidget`) false false)
  (`KismetSystemLibrary.Delay` 5.0)
  (bind _returnvalue (`GameplayStatics.GetCurrentLevelName` true))
  (`GameplayStatics.OpenLevel` (`KismetStringLibrary.Conv_StringToName` _returnvalue)))

(event `self.ReceiveTick`
  (params (DeltaSeconds :type "Float (single-precision)"))
  (bind _energyf (`self.EnergyF`))
  (if (== (`self.EnergyF`) 0.0)
    (`self.Lose`)
    (elif (== (`self.DefectsCount`) 0.0)
      (`self.Win`)
      (elif (<= _energyf (+ (`self.MaxEnergy`) (`self.Charging speed`)))
        (set `self.EnergyF` (+ _energyf (`self.Is charging`)))
        (else
          (set `self.EnergyF` (`self.MaxEnergy`)))))))

(event `Win`
  (`SceneComponent.SetHiddenInGame` (`self.WinWidget`) false false)
  (`KismetSystemLibrary.Delay` 5.0)
  (`GameplayStatics.OpenLevel` "Main_Menu"))

(event `OnChargeStart`
  (set `self.Is charging` (`self.Charging speed`)))

(event `InputAxis|ForwardMovingAxis`
  (params (AxisValue :type "Float (single-precision)"))
  (`self.AddMovementInput` (`SceneComponent.GetForwardVector` (`self.Camera`)) AxisValue))

(event `OnChargeEnd`
  (set `self.Is charging` (`self.Uncharging speed`)))

(event `InputAxis|RightMovingAxis`
  (params (AxisValue :type "Float (single-precision)"))
  (`self.AddMovementInput` (`SceneComponent.GetRightVector` (`self.Camera`)) AxisValue))

(event `InputAction|Grib_L`
  (params (Key :type "Key Structure"))
  (:`Pressed`
    (set `self.IsGrab` true)
    (bind _outactors (`KismetSystemLibrary.SphereOverlapActors` (`SceneComponent.K2_GetComponentLocation` (`self.SkeletalMesh`)) 10.0 (`|MakeArray` "ObjectTypeQuery2" "ObjectTypeQuery4" "ObjectTypeQuery1" :!type "EObjectTypeQuery Enum") null (`|MakeArray` self :!type "Actor Object Reference")))
    (bind _output_get (set `self.GrabedActor` (`|GetArrayItem` _outactors)))
    (message `/Game/VR/Player/Interfaces/IF_VRInteraction.Grab` _output_get self))
  (:`Released`
    (set `self.IsGrab` false)
    (message `/Game/VR/Player/Interfaces/IF_VRInteraction.UnGrab` (`self.GrabedActor`) self)
    (set `self.GrabedActor` null)))

(event `InputAction|MenuAction`
  (params (Key :type "Key Structure"))
  (bind _widgetinteraction (`self.WidgetInteraction`))
  (:`Pressed`
    (`WidgetInteractionComponent.PressPointerKey` _widgetinteraction "LeftMouseButton"))
  (:`Released`
    (`WidgetInteractionComponent.ReleasePointerKey` _widgetinteraction "LeftMouseButton")))

(event `InputAction|OpenMenu`
  (params (Key :type "Key Structure"))
  (bind _widgetinteraction (`self.WidgetInteraction`))
  (bind _widget (`self.Widget`))
  (:`Pressed`
    (`/Engine/EditorBlueprintResources/StandardMacros.FlipFlop`
      (:`A`
        (set `WidgetInteractionComponent.bShowDebug` true _widgetinteraction)
        (`SceneComponent.SetHiddenInGame` _widget false false))
      (:`B`
        (set `WidgetInteractionComponent.bShowDebug` false _widgetinteraction)
        (`SceneComponent.SetHiddenInGame` _widget true false)))))

(event `InputAction|Trigger_R`
  (params (Key :type "Key Structure"))
  (bind _arrow1 (`self.Arrow1`))
  (:`Pressed`
    (bind (_outhit _returnvalue) (`KismetSystemLibrary.CapsuleTraceSingle` (`SceneComponent.K2_GetComponentLocation` _arrow1) (* (`SceneComponent.GetForwardVector` _arrow1) 10000.0) 0.0 0.0 "TraceTypeQuery1"))
    (if _returnvalue
      (bind (_bblockinghit _binitialoverlap _time _distance _location _impactpoint _normal _impactnormal _physmat _hitactor) (`GameplayStatics.BreakHitResult` _outhit))
      (if (`KismetSystemLibrary.DoesImplementInterface` _hitactor "/Game/VR/Player/Interfaces/IF_VRInteraction.IF_VRInteraction_C")
        (bind _yes (message `/Game/VR/Player/Interfaces/IF_VRInteraction.CanRepair` _hitactor))
        (if _yes
          (set `self.TargetActor` _hitactor)
          (`SceneComponent.SetVisibility` (`self.ParticleSystem`) true false)
          (`KismetSystemLibrary.Delay` 2.0)
          (bind _targetactor (`self.TargetActor`)
            (:`then`
              (bind _ok (message `/Game/VR/Player/Interfaces/IF_VRInteraction.Use` _targetactor self))
              (if _ok
                (set `self.DefectsCount` (- (`self.DefectsCount`) 1.0))
                (set `self.TargetActor` null)
                (`SceneComponent.SetVisibility` (`self.ParticleSystem`) false false)))
            (:`else`))))))
  (:`Released`
    (bind _targetactor_2 (`self.TargetActor`)
      (:`then`
        (message `/Game/VR/Player/Interfaces/IF_VRInteraction.UnUse` _targetactor_2 self)
        (set `self.TargetActor` null)
        (`SceneComponent.SetVisibility` (`self.ParticleSystem`) false false))
      (:`else`))))

(fn `GetZ`
  (returns (Z :type "Float (double-precision)"))
  (bind (_returnvalue_x _returnvalue_y _returnvalue_z) (`KismetMathLibrary.BreakVector` (`SceneComponent.K2_GetComponentLocation` (`self.Camera`))))
  (return (/ (- 100.0 _returnvalue_z) 100.0)))

(fn `UserConstructionScript`)